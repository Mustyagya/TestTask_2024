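; BP_Task_01_Actor is an actor whose sphere changes material when another actor overlaps its collision sphere.
; On begin overlap it sends overlap and player flags as true to the other actor through message calls, reads them back, and applies the red material if both hold.
; Any end overlap applies BasicAsset03, without checking the actor.
; Its own Get/Set overlap functions are empty.
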(event OnComponentBeginOverlap(Sphere_Col)
  (params (OverlappedComponent :type Primitive%20Component%20Object%20Reference) (OtherActor :type Actor%20Object%20Reference) (OtherComp :type Primitive%20Component%20Object%20Reference) (OtherBodyIndex :type Integer) (bFromSweep :type Boolean) (SweepResult :type Hit%20Result%20Structure%20%28by%20ref%29))
  (Variables|Default|SetOther%20Actor OtherActor)
  (Class|BPTaskO1Interface|SetIsOverlapp(Message) (Variables|Default|GetOther%20Actor) true true)
  (bind (_is__overlepping _is_player) (Class|BPTaskO1Interface|GetIsOverlapp(Message) (Variables|Default|GetOther%20Actor)))
  (if _is__overlepping
    (if _is_player
      (CallFunction|ChangeColor))))

(event OnComponentEndOverlap(Sphere_Col)
  (params (OverlappedComponent :type Primitive%20Component%20Object%20Reference) (OtherActor :type Actor%20Object%20Reference) (OtherComp :type Primitive%20Component%20Object%20Reference) (OtherBodyIndex :type Integer))
  (Rendering|Material|CreateDynamicMaterialInstance (Variables|Default|GetSphere) 0 "/Engine/MapTemplates/Materials/BasicAsset03.BasicAsset03" "None" :!class /Script/Engine.PrimitiveComponent))

(event Custom|Change%20color
  (Rendering|Material|CreateDynamicMaterialInstance (Variables|Default|GetSphere) 0 "/AnimationSharing/AnimSharingRed.AnimSharingRed" "None" :!class /Script/Engine.PrimitiveComponent))

(event EventBeginPlay)

(event Collision|EventActorBeginOverlap
  (params (OtherActor :type Actor%20Object%20Reference)))

(event EventTick
  (params (DeltaSeconds :type Float%20%28single-precision%29)))

(fn ConstructionScript)

(fn GetIsOverlapp)

(fn SetIsOverlapp
  (params (B%20SetOverLepping :type Boolean) (Is%20Player :type Boolean)))